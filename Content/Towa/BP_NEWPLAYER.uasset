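; Player Blueprint that orbits its spring-arm camera with the mouse while the right button is held.
; Right-click sets a flag and samples input axis values through SetMousePrevPos.
; While flagged, Tick applies the stored values scaled by CameraSpeed as world yaw and relative pitch, then resamples.
; Pitch is clamped to a downward-looking range, and no movement or other gameplay logic is present.
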(event `Key|RightMouseButton`
  (params (Key :type "Key Structure"))
  ; クリックを押しているかのフラグ
  (:`Pressed`
    (set `self.isRightClicking` true)
    (`self.SetMousePrevPos`))
  (:`Released`
    (set `self.isRightClicking` false)))

(event `self.ReceiveTick`
  (params (DeltaSeconds :type "Float (single-precision)"))
  (bind _cameraspeed (`self.CameraSpeed`))
  (bind _springarm (`self.SpringArm`))
  ; カメラの回転処理
  (if (`self.isRightClicking`)
    (`SceneComponent.K2_AddWorldRotation` _springarm (`KismetMathLibrary.MakeRotator` 0.0 0.0 (* (`self.prevMouseX`) _cameraspeed)) false false)
    (`SceneComponent.K2_SetRelativeRotation` _springarm (`KismetMathLibrary.MakeRotator` (.roll (`SpringArmComponent.GetTargetRotation` _springarm)) (`KismetMathLibrary.FClamp` (+ (* (`self.PrevMouseY`) _cameraspeed) (.pitch (`SpringArmComponent.GetTargetRotation` _springarm))) -75.0 -20.0) (.yaw (`SpringArmComponent.GetTargetRotation` _springarm))) false false)
    (`self.SetMousePrevPos`)))

(fn `SetMousePrevPos`
  ; マウスの履歴を更新する関数
  (set `self.prevMouseX` (`self.GetInputAxisKeyValue`))
  (set `self.PrevMouseY` (`self.GetInputAxisKeyValue`)))

(fn `UserConstructionScript`)